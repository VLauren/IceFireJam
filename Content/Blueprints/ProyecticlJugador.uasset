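; Player projectile Blueprint that damages enemies on contact.
; Each Tick it moves itself along its Arrow's forward vector at VelocidadDisparo per frame, without sweep or delta-time scaling.
; Sphere overlaps deal 10 damage to Enemy actors, then destroy the projectile after a brief delay.
; A cast chain ignores both player projectile types, PJ_1n and PJ_2; any other actor also destroys it.
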(event OnComponentBeginOverlap(Sphere)
  (params (OverlappedComponent :type Primitive%20Component%20Object%20Reference) (OtherActor :type Actor%20Object%20Reference) (OtherComp :type Primitive%20Component%20Object%20Reference) (OtherBodyIndex :type Integer) (bFromSweep :type Boolean) (SweepResult :type Hit%20Result%20Structure%20%28by%20ref%29))
  (bind _asenemy (Utilities|Casting|CastToEnemy OtherActor)
    (:then
      (Default|Damage _asenemy 10))
    (:CastFailed
      (Utilities|Casting|CastToProyecticlJugador OtherActor
        (:CastFailed
          (Utilities|Casting|CastToProyecticlJugador2 OtherActor
            (:CastFailed
              (Utilities|Casting|CastToPJ_1n OtherActor
                (:CastFailed
                  (Utilities|Casting|CastToPJ_2 OtherActor
                    (:CastFailed
                      _))))))))))
  (Utilities|FlowControl|Delay 0.01)
  (Actor|DestroyActor))

(event EventTick
  (params (DeltaSeconds :type Float%20%28single-precision%29))
  (Transformation|SetActorLocation (+ (Transformation|GetActorLocation) (* (Math|Vector|GetForwardVector (Variables|Default|GetArrow)) (Variables|Default|GetVelocidadDisparo))) false false))

(fn ConstructionScript)
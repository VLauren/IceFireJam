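; Player actor (jugador1) that fires projectiles and defines four WASD-named movement functions.
; Left mouse press spawns a ProyecticlJugador at the Arrow component's world transform.
; Each movement function checks its flag and offsets world X or Y by the Arrow's forward component plus or minus a fixed step; the "girar" functions translate rather than rotate.
; The event graph neither calls these functions nor sets their flags.
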(event Input|MouseEvents|LeftMouseButton
  (params (Key :type Key%20Structure))
  (:Pressed
    (Game|SpawnActorfromClass "/Game/Blueprints/ProyecticlJugador.ProyecticlJugador_C" (Transformation|GetWorldTransform (Variables|Default|GetArrow)) "Undefined" 0 0)))

(fn ConstructionScript)

(fn MoverhaciaAlante
  (if (Variables|Default|Getw)
    (Transformation|AddActorWorldOffset (Math|Vector|MakeVector (+ (.x (Math|Vector|GetForwardVector (Variables|Default|GetArrow))) 5.0) 0.0 0.0))))

(fn MoverHaciaAtras
  (if (Variables|Default|Gets)
    (Transformation|AddActorWorldOffset (Math|Vector|MakeVector (- (.x (Math|Vector|GetForwardVector (Variables|Default|GetArrow))) 5.0) 0.0 0.0))))

(fn Girarizquierda
  (if (Variables|Default|Geta)
    (Transformation|AddActorWorldOffset (Math|Vector|MakeVector 0.0 (- (.y (Math|Vector|GetForwardVector (Variables|Default|GetArrow))) 5.0) 0.0))))

(fn GirarDerecha
  (if (Variables|Default|Getd)
    (Transformation|AddActorWorldOffset (Math|Vector|MakeVector 0.0 (+ (.y (Math|Vector|GetForwardVector (Variables|Default|GetArrow))) 5.0) 0.0))))
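; ProyecticlJugador2 is a player projectile, apparently player two's, that damages enemies.
; Each Tick it moves without sweep along its Arrow's forward vector by VelocidadDisparo, not scaled by delta time.
; The first Sphere overlap, gated by DoOnce, damages an Enemy, then destroys the projectile after a tiny delay whatever it hit.
; Cast checks for filtering players and other projectiles are left disconnected and never run.
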(event OnComponentBeginOverlap(Sphere)
  (params (OverlappedComponent :type Primitive%20Component%20Object%20Reference) (OtherActor :type Actor%20Object%20Reference) (OtherComp :type Primitive%20Component%20Object%20Reference) (OtherBodyIndex :type Integer) (bFromSweep :type Boolean) (SweepResult :type Hit%20Result%20Structure%20%28by%20ref%29))
  (Utilities|FlowControl|DoOnce false
    (:Completed
      (Utilities|FlowControl|Sequence
        (:then_0
          (bind _asenemy (Utilities|Casting|CastToEnemy OtherActor))
          (Default|Damage _asenemy 10))
        (:then_1
          _))
      (Utilities|FlowControl|Delay 0.01)
      (Actor|DestroyActor))))

(event EventTick
  (params (DeltaSeconds :type Float%20%28single-precision%29))
  (Transformation|SetActorLocation (+ (Transformation|GetActorLocation) (* (Math|Vector|GetForwardVector (Variables|Default|GetArrow)) (Variables|Default|GetVelocidadDisparo))) false false))

(fn ConstructionScript)
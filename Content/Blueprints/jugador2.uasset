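; Second-player Blueprint (jugador2) with directional movement helpers and a projectile-firing graph that is not connected to any event.
; Four functions, gated by direction booleans, nudge the actor along world X or Y by the Arrow's forward component plus or minus a constant; the "girar" pair translates rather than rotates.
; Nothing shown calls these functions, and the unwired DoOnce spawn of ProyecticlJugador and its delayed reset never run.
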(event Input|KeyboardEvents|Enter
  (params (Key :type Key%20Structure)))

(fn ConstructionScript)

(fn MoverhaciaAlante
  (if (Variables|Default|Getarriba)
    (Transformation|AddActorWorldOffset (Math|Vector|MakeVector (+ (.x (Math|Vector|GetForwardVector (Variables|Default|GetArrow))) 5.0) 0.0 0.0))))

(fn MoverHaciaAtras
  (if (Variables|Default|Getabajo)
    (Transformation|AddActorWorldOffset (Math|Vector|MakeVector (- (.x (Math|Vector|GetForwardVector (Variables|Default|GetArrow))) 5.0) 0.0 0.0))))

(fn Girarizquierda
  (if (Variables|Default|Getizquierda)
    (Transformation|AddActorWorldOffset (Math|Vector|MakeVector 0.0 (- (.y (Math|Vector|GetForwardVector (Variables|Default|GetArrow))) 5.0) 0.0))))

(fn GirarDerecha
  (if (Variables|Default|Getright)
    (Transformation|AddActorWorldOffset (Math|Vector|MakeVector 0.0 (+ (.y (Math|Vector|GetForwardVector (Variables|Default|GetArrow))) 5.0) 0.0))))
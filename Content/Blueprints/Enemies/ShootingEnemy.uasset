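; ShootingEnemy is an enemy that chases player one and periodically fires a projectile.
; Tick runs a timer-driven state machine that loops through Idle, Chasing and Attacking, moving toward the player only while Chasing.
; When the chase timer expires, Shoot spawns an EnemyProjectile offset along the actor's forward vector, then Attacking serves as a short pause before Idle.
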(event EventTick
  (params (DeltaSeconds :type Float%20%28single-precision%29))
  (|CallParentFunction DeltaSeconds)
  (Variables|Default|SetCounter (+ (Variables|Default|GetCounter) (Variables|Default|GetdeltaTime)))
  (switch Utilities|FlowControl|Switch|SwitchonEnemyStates (Variables|Default|GetEnemyState)
    (:NewEnumerator0
      ;[1 1 1] Idle
      (if (>= (Variables|Default|GetCounter) 0.5)
        (Variables|Default|SetCounter 0.0)
        (Variables|Default|SetEnemyState "NewEnumerator1")))
    (:NewEnumerator1
      ;[1 1 1] Chasing
      (bind _playerposition (CallFunction|GetPlayer1Location))
      (CallFunction|MoveTowards (Variables|Default|GetdeltaTime) _playerposition 2e+02)
      (if (>= (Variables|Default|GetCounter) 3.0)
        (CallFunction|Shoot)
        (Variables|Default|SetCounter 0.0)
        (Variables|Default|SetEnemyState "NewEnumerator2")))
    (:NewEnumerator2
      ;[1 1 1] Attacking
      (if (>= (Variables|Default|GetCounter) 1.0)
        (Variables|Default|SetCounter 0.0)
        (Variables|Default|SetEnemyState "NewEnumerator0")))))

(fn ConstructionScript
  (|CallParentFunction))

(fn Shoot
  (bind _returnvalue (Game|SpawnActorfromClass "/Game/Blueprints/Enemies/Projectiles/EnemyProjectile.EnemyProjectile_C" (Transformation|GetActorTransform) "Undefined" 0 0))
  (Transformation|SetActorLocation _returnvalue (+ (Transformation|GetActorLocation) (* (Transformation|GetActorForwardVector) 1e+02)) false false))
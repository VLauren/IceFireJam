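; Kamikaze enemy with one hit point that chases the nearest player and damages it on contact.
; Each tick it moves its Collision in X and Y toward that player with random jitter, unscaled by delta time.
; The look-at direction is multiplied by zero, so rotation does not track the target.
; Box overlap with either player class, PJ_1n or PJ_2, deals a heavy hit, then destroys the enemy after a short delay.
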(event OnComponentBeginOverlap(Box)
  (params (OverlappedComponent :type Primitive%20Component%20Object%20Reference) (OtherActor :type Actor%20Object%20Reference) (OtherComp :type Primitive%20Component%20Object%20Reference) (OtherBodyIndex :type Integer) (bFromSweep :type Boolean) (SweepResult :type Hit%20Result%20Structure%20%28by%20ref%29))
  (Utilities|FlowControl|Sequence
    (:then_0
      (bind _aspj_2 (Utilities|Casting|CastToPJ_2 OtherActor))
      (Default|Hit _aspj_2 100))
    (:then_1
      (bind _aspj_1n (Utilities|Casting|CastToPJ_1n OtherActor))
      (Default|Hit _aspj_1n 100)))
  (Utilities|FlowControl|Delay 0.2)
  (Actor|DestroyActor))

(event EventBeginPlay
  (|CallParentFunction)
  (Variables|Default|SetMaxHp 1))

(event EventTick
  (params (DeltaSeconds :type Float%20%28single-precision%29))
  (|CallParentFunction DeltaSeconds)
  (bind _playerposition (CallFunction|GetNearestPlayerLocation))
  (Transformation|SetWorldRotation (Variables|Default|GetCollision) (Math|Conversions|RotationFromXVector (* (- _playerposition (Transformation|GetWorldLocation (Variables|Default|GetCollision))) 0.0)) false false)
  (Transformation|AddRelativeLocation (Variables|Default|GetCollision) (Math|Vector|MakeVector (+ (.x (* (Math|Vector|Normalize (- _playerposition (Transformation|GetWorldLocation (Variables|Default|GetCollision)))) (Variables|Default|GetMovementSpeed))) (Math|Random|RandomFloatinRange -3.0 3.0)) (+ (.y (* (Math|Vector|Normalize (- _playerposition (Transformation|GetWorldLocation (Variables|Default|GetCollision)))) (Variables|Default|GetMovementSpeed))) (Math|Random|RandomFloatinRange -3.0 3.0)) 0.0) false false))

(fn ConstructionScript
  (|CallParentFunction))
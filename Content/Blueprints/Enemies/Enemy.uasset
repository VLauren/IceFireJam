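; Enemy actor for a two-player game that provides player lookup, movement and damage functions, though nothing in this file calls them.
; BeginPlay caches the first Jugador1 and Jugador2, and Tick only stores delta time.
; MoveTowards does a swept horizontal step and faces the destination, while GetNearestPlayerLocation actually returns the farther player because its comparison is inverted.
; Damage prints the amount and destroys the enemy on any hit.
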(event EventBeginPlay
  (bind _outactors (Actor|GetAllActorsOfClass "/Game/Blueprints/jugador1.jugador1_C"))
  (Variables|Default|SetPlayer1 (Utilities|Array|Get(acopy) _outactors))
  (bind _outactors_2 (Actor|GetAllActorsOfClass "/Game/Blueprints/jugador2.jugador2_C"))
  (Variables|Default|SetPlayer2 (Utilities|Array|Get(acopy) _outactors_2)))

(event EventTick
  (params (DeltaSeconds :type Float%20%28single-precision%29))
  (Variables|Default|SetdeltaTime DeltaSeconds))

(fn ConstructionScript)

(fn Damage
  (params (Damage :type Integer))
  (Development|PrintString (Utilities|String|Append "Enemigo recibe daño: " (Utilities|String|ToString(Integer) Damage)))
  (Actor|DestroyActor))

(fn GetPlayer1Location
  (return (Transformation|GetActorLocation (Variables|Default|GetPlayer1))))

(fn GetPlayer2Location
  (return (Transformation|GetActorLocation (Variables|Default|GetPlayer2))))

(fn GetNearestPlayerLocation
  (bind _player1 (Variables|Default|GetPlayer1))
  (bind _player2 (Variables|Default|GetPlayer2))
  (bind _returnvalue (Transformation|GetActorLocation _player2))
  (bind _returnvalue_2 (Transformation|GetActorLocation _player1))
  (if (> (Math|Vector|VectorLengthSquared (- _returnvalue_2 (Transformation|GetActorLocation))) (Math|Vector|VectorLengthSquared (- _returnvalue (Transformation|GetActorLocation))))
    (return _returnvalue_2)
    (else
      (return _returnvalue))))

(fn MoveTowards
  (params (DeltaTime :type Float%20%28single-precision%29) (Destination :type Vector) (MovementSpeed :type Float%20%28single-precision%29))
  (bind _returnvalue (Transformation|GetActorLocation))
  (bind _returnvalue_2 (- Destination _returnvalue))
  (bind _returnvalue_3 (Math|Vector|Normalize _returnvalue_2))
  (bind (_x _y) (Math|Vector|BreakVector _returnvalue_3))
  (bind _returnvalue_4 (* _returnvalue_3 MovementSpeed))
  (bind _returnvalue_5 (* _returnvalue_4 DeltaTime))
  (bind (_x_2 _y_2) (Math|Vector|BreakVector _returnvalue_5))
  (Transformation|SetActorLocation (+ (Math|Vector|MakeVector _x_2 _y_2 0.0) _returnvalue) true false)
  (Transformation|SetActorRotation (Math|Conversions|RotationFromXVector (Math|Vector|MakeVector _x _y 0.0))))
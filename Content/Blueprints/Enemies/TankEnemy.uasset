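; Tank enemy for a two-player game that patrols, chases the nearest player and deals a heavy hit to either on overlap.
; A Tick state machine goes from a brief Idle to Patrol, then to Chasing once a player is near, with no way back.
; Patrol moves between random navigable points, repicking on arrival or when a position-based timer detects it is stuck.
; Point selection rerolls only once if the point is too high.
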(event Collision|EventActorBeginOverlap
  (params (OtherActor :type Actor%20Object%20Reference))
  (bind _player1 (Variables|Default|GetPlayer1))
  (bind _player2 (Variables|Default|GetPlayer2))
  (if (== OtherActor _player1)
    (Default|Hit _player1 100)
    (elif (== OtherActor _player2)
      (Default|Hit _player2 100))))

(event EventTick
  (params (DeltaSeconds :type Float%20%28single-precision%29))
  (bind _returnvalue (Transformation|GetActorLocation))
  (bind _nextpatroldestination (Variables|Default|GetNextPatrolDestination))
  (bind (_x _y) (Math|Vector|BreakVector _returnvalue))
  (bind (_x_2 _y_2) (Math|Vector|BreakVector _nextpatroldestination))
  (|CallParentFunction DeltaSeconds)
  (Variables|Default|SetCounter (+ (Variables|Default|GetCounter) (Variables|Default|GetdeltaTime)))
  (switch Utilities|FlowControl|Switch|SwitchonEnemyStates (Variables|Default|GetEnemyState)
    (:NewEnumerator0
      (if (>= (Variables|Default|GetCounter) 0.5)
        (Variables|Default|SetCounter 0.0)
        (Variables|Default|SetEnemyState "NewEnumerator3")
        (CallFunction|FindNextPatrolPoint)))
    (:NewEnumerator3
      (CallFunction|MoveTowards (Variables|Default|GetdeltaTime) (Variables|Default|GetNextPatrolDestination) (Variables|Default|GetMovementSpeed))
      (if (or (> (Variables|Default|GetTiempoSinMovimiento) 1.5) (< (Math|Vector|VectorLength (- (Math|Vector|MakeVector _x _y 0.0) (Math|Vector|MakeVector _x_2 _y_2 0.0))) 1e+02))
        (CallFunction|FindNextPatrolPoint)
        (Variables|Default|SetTiempoSinMovimiento 0.0)
        (else
          (if (Math|Vector|Equal(Vector) (Variables|Default|GetUltimaPos) (Transformation|GetActorLocation) 1e+01)
            (Variables|Default|SetTiempoSinMovimiento (+ (Variables|Default|GetTiempoSinMovimiento) (Variables|Default|GetdeltaTime)))
            (else
              (Variables|Default|SetTiempoSinMovimiento 0.0)))
          (Variables|Default|SetUltimaPos (Transformation|GetActorLocation))))
      (bind _playerposition (CallFunction|GetNearestPlayerLocation))
      (if (<= (Math|Vector|VectorLength (- _playerposition (Transformation|GetActorLocation))) 5e+02)
        (Variables|Default|SetCounter 0.0)
        (Variables|Default|SetEnemyState "NewEnumerator1")))
    (:NewEnumerator1
      (bind _playerposition_2 (CallFunction|GetNearestPlayerLocation))
      (CallFunction|MoveTowards (Variables|Default|GetdeltaTime) _playerposition_2 (Variables|Default|GetMovementSpeed)))))

(fn ConstructionScript
  (|CallParentFunction))

(fn FindNextPatrolPoint
  (Variables|Default|SetNextPatrolDestination (.RandomLocation (Class|NavigationSystemV1|GetRandomPointinNavigableRadius (Transformation|GetActorLocation) 5e+02 0 0)))
  (while (> (.z (Variables|Default|GetNextPatrolDestination)) 6e+01)
    (Variables|Default|SetNextPatrolDestination (.RandomLocation (Class|NavigationSystemV1|GetRandomPointinNavigableRadius (Transformation|GetActorLocation) 5e+02 0 0)))
    (return)))
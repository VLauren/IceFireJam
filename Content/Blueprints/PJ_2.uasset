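; PJ_2 is an actor, apparently the second player character, that reports its death to the GM_FuegoHielo game mode.
; Hit ignores its Damage input, takes one life from the game mode's Vidas, sets the PJ2 flag, calls QuedanVidas and destroys the actor.
; Keys 1 and 2 call LevelDOWN and LevelUP on the same game mode.
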(event Collision|EventActorBeginOverlap
  (params (OtherActor :type Actor%20Object%20Reference)))

(event EventTick
  (params (DeltaSeconds :type Float%20%28single-precision%29)))

(event Input|KeyboardEvents|1
  (params (Key :type Key%20Structure))
  (:Pressed
    (bind _asgm_fuego_hielo (Utilities|Casting|CastToGM_FuegoHielo (Game|GetGameMode)))
    (Default|LevelDOWN _asgm_fuego_hielo)))

(event Input|KeyboardEvents|2
  (params (Key :type Key%20Structure))
  (:Pressed
    (bind _asgm_fuego_hielo (Utilities|Casting|CastToGM_FuegoHielo (Game|GetGameMode)))
    (Default|LevelUP _asgm_fuego_hielo)))

(fn ConstructionScript)

(fn Hit
  (params (Damage :type Integer))
  (Development|PrintString "HIT")
  (bind _asgm_fuego_hielo (Utilities|Casting|CastToGM_FuegoHielo (Game|GetGameMode)))
  (Variables|/Game/Blueprints/GM_FuegoHielo.GM_FuegoHielo_C|SetVidas _asgm_fuego_hielo (- (Variables|/Game/Blueprints/GM_FuegoHielo.GM_FuegoHielo_C|GetVidas _asgm_fuego_hielo) 1))
  (Variables|/Game/Blueprints/GM_FuegoHielo.GM_FuegoHielo_C|SetPJ2 _asgm_fuego_hielo true)
  (Default|QuedanVidas? _asgm_fuego_hielo)
  (Actor|DestroyActor))
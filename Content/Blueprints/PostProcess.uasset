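; Post-process controller that turns a signed heat/cold Stage value into escalating screen effects and end states.
; StageUpdate branches on Stage: negative values lower the Cold volume's color temperature, positive ones raise the Heat volume's color gain and an intensity, zero restores neutral.
; Intermediate stages toggle the Cold1/Heat1 volumes and particles.
; At either extreme, it shows the matching end widget and pauses the game.
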(event Custom|StageUpdate
  (bind _stage (Variables|Default|GetStage))
  (bind _stage_2 (Variables|Default|GetStage))
  (Development|PrintString (Utilities|String|ToString(Integer) _stage))
  (if (== _stage -5)
    (bind _returnvalue (UserInterface|CreateWidget "/Game/Widgets/Widg_End_Cold.Widg_End_Cold_C"))
    (UserInterface|Viewport|AddtoViewport _returnvalue 0)
    (Game|SetGamePaused true)
    (elif (== _stage -4)
      (Utilities|Struct|SetmembersinPostProcessSettings (Variables|/Script/Engine.PostProcessComponent|GetSettings (Variables|Default|GetCold)) 4.5e+03 0.0)
      (elif (== _stage -3)
        (Utilities|Struct|SetmembersinPostProcessSettings (Variables|/Script/Engine.PostProcessComponent|GetSettings (Variables|Default|GetCold)) 5166.0 0.0)
        (Variables|/Script/Engine.PostProcessComponent|SetbEnabled (Variables|Default|GetCold1) true)
        (elif (== _stage -2)
          (Components|Activation|Activate (Variables|Default|GetParticle_Cold) false)
          (elif (== _stage -1)
            (Utilities|Struct|SetmembersinPostProcessSettings (Variables|/Script/Engine.PostProcessComponent|GetSettings (Variables|Default|GetCold)) 5832.0 0.0)
            (Variables|/Script/Engine.PostProcessComponent|SetbEnabled (Variables|Default|GetCold1) false)
            (Components|Activation|Deactivate (Variables|Default|GetParticle_Cold))
            (elif (== _stage_2 0)
              (Utilities|Struct|SetmembersinPostProcessSettings (Variables|/Script/Engine.PostProcessComponent|GetSettings (Variables|Default|GetCold)) 6.5e+03)
              (Utilities|Struct|SetmembersinPostProcessSettings (Variables|/Script/Engine.PostProcessComponent|GetSettings (Variables|Default|GetHeat)) 6.5e+03 (Math|Vector4|MakeVector4 1.0 1.0 1.0 1.0))
              (elif (== _stage_2 1)
                (Utilities|Struct|SetmembersinPostProcessSettings (Variables|/Script/Engine.PostProcessComponent|GetSettings (Variables|Default|GetHeat)) (Math|Vector4|MakeVector4 1.26 1.08 0.93 1.073) 1.775)
                (Variables|/Script/Engine.PostProcessComponent|SetbEnabled (Variables|Default|GetHeat1) false)
                (Components|Activation|Deactivate (Variables|Default|GetParticle_Heat))
                (elif (== _stage_2 2)
                  (Components|Activation|Activate (Variables|Default|GetParticle_Heat) false)
                  (elif (== _stage_2 3)
                    (Utilities|Struct|SetmembersinPostProcessSettings (Variables|/Script/Engine.PostProcessComponent|GetSettings (Variables|Default|GetHeat)) (Math|Vector4|MakeVector4 1.6 1.17 0.86 1.146) 2.9)
                    (Variables|/Script/Engine.PostProcessComponent|SetbEnabled (Variables|Default|GetHeat1) true)
                    (elif (== _stage_2 4)
                      (Utilities|Struct|SetmembersinPostProcessSettings (Variables|/Script/Engine.PostProcessComponent|GetSettings (Variables|Default|GetHeat)) (Math|Vector4|MakeVector4 1.8 1.25 0.79 1.22) 4.0)
                      (elif (== _stage_2 5)
                        (bind _returnvalue_2 (UserInterface|CreateWidget "/Game/Widgets/Widg_End_Hot.Widg_End_Hot_C"))
                        (UserInterface|Viewport|AddtoViewport _returnvalue_2 0)
                        (Game|SetGamePaused true)))))))))))))

(fn ConstructionScript)
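; Central input controller for local two-player play, driving PJ_1n with WASD and Space, and PJ_2 with mapped directional actions plus Enter or a gamepad face button.
; Input events set direction and movement flags, which Tick uses to offset both characters with sweep and snap their yaw, including diagonals.
; Firing spawns a projectile at the character's Arrow through a resettable DoOnce and shifts GM_FuegoHielo's Temperatura down for player one, up for player two.
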(event EventBeginPlay
  (bind _outactors (Actor|GetAllActorsOfClass "/Game/Blueprints/PJ_1n.PJ_1n_C"))
  (Variables|Default|SetRefPJ1 (Utilities|Array|Get(acopy) _outactors))
  (bind _outactors_2 (Actor|GetAllActorsOfClass "/Game/Blueprints/PJ_2.PJ_2_C"))
  (Variables|Default|SetPJ2 (Utilities|Array|Get(acopy) _outactors_2)))

(event EventTick
  (params (DeltaSeconds :type Float%20%28single-precision%29))
  (Utilities|FlowControl|Sequence
    (:then_0
      (CallFunction|Jugador1alante))
    (:then_1
      (CallFunction|Jugador1detras))
    (:then_2
      (CallFunction|Jugador1izquierda))
    (:then_3
      (CallFunction|Jugador1derecha))
    (:then_4
      (CallFunction|Jugador2arriba))
    (:then_5
      (CallFunction|Jugador2abajo))
    (:then_6
      (CallFunction|Jugador2izquierda))
    (:then_7
      (CallFunction|Jugador2derecha))
    (:then_8
      (CallFunction|Jugador1arribaderecha))
    (:then_9
      (if (Math|Boolean|ORBoolean (Variables|Default|Getd) (Variables|Default|Geta) (Variables|Default|Getw) (Variables|Default|Gets))
        (Variables|Default|SetmovimientoPJ1 true)))
    (:then_10
      (if (Math|Boolean|ORBoolean (Variables|Default|Getizquierda) (Variables|Default|Getright) (Variables|Default|Getarriba) (Variables|Default|Getabajo))
        (Variables|Default|SetMovimientoPj2 true)))))

(event Input|ActionEvents|InputActionderechaMando/teclado
  (params (Key :type Key%20Structure))
  (:Pressed
    (Variables|Default|Setright true)
    (Variables|Default|SetMovimientoPj2 true))
  (:Released
    (Variables|Default|Setright false)
    (Variables|Default|SetMovimientoPj2 false)))

(event Input|ActionEvents|InputActionIzquierdaMando/teclado
  (params (Key :type Key%20Structure))
  (:Pressed
    (Variables|Default|Setizquierda true)
    (Variables|Default|SetMovimientoPj2 true))
  (:Released
    (Variables|Default|Setizquierda false)
    (Variables|Default|SetMovimientoPj2 false)))

(event Input|ActionEvents|InputActionarribaMando/teclado
  (params (Key :type Key%20Structure))
  (:Pressed
    (Variables|Default|Setarriba true)
    (Variables|Default|SetMovimientoPj2 true))
  (:Released
    (Variables|Default|Setarriba false)
    (Variables|Default|SetMovimientoPj2 false)))

(event Input|ActionEvents|InputActionabajoMando/teclado
  (params (Key :type Key%20Structure))
  (:Pressed
    (Variables|Default|Setabajo true)
    (Variables|Default|SetMovimientoPj2 true))
  (:Released
    (Variables|Default|Setabajo false)
    (Variables|Default|SetMovimientoPj2 false)))

(event Input|KeyboardEvents|W
  (params (Key :type Key%20Structure))
  (:Pressed
    (Variables|Default|Setw true)
    (Variables|Default|SetmovimientoPJ1 true))
  (:Released
    (Variables|Default|Setw false)
    (Variables|Default|SetmovimientoPJ1 false)))

(event Input|KeyboardEvents|SpaceBar
  (params (Key :type Key%20Structure))
  (:Pressed
    (Variables|Default|SetDisparoPJ1 true)
    (Utilities|FlowControl|DoOnce false :!label _label
      (:Completed
        (Game|SpawnActorfromClass "/Game/Blueprints/ProyecticlJugador.ProyecticlJugador_C" (Transformation|GetWorldTransform (Variables|/Game/Blueprints/PJ_1n.PJ_1n_C|GetArrow (Variables|Default|GetRefPJ1))) "Undefined" 0 0)
        (bind _asgm_fuego_hielo (Utilities|Casting|CastToGM_FuegoHielo (Game|GetGameMode)))
        (Variables|/Game/Blueprints/GM_FuegoHielo.GM_FuegoHielo_C|SetTemperatura _asgm_fuego_hielo (- (Variables|/Game/Blueprints/GM_FuegoHielo.GM_FuegoHielo_C|GetTemperatura _asgm_fuego_hielo) (Variables|Default|Gethielito)))
        (Utilities|FlowControl|Delay 0.2)
        (Variables|Default|SetDisparoPJ1 false))))
  (:Released
    (Utilities|FlowControl|Delay 0.01)
    (goto _label Reset)))

(event Input|GamepadEvents|GamepadFaceButtonBottom
  (params (Key :type Key%20Structure))
  (:Pressed
    (Variables|Default|SetDisparoPJ2 true)
    (Utilities|FlowControl|DoOnce false :!label _label
      (:Completed
        (Game|SpawnActorfromClass "/Game/Blueprints/ProyecticlJugador2.ProyecticlJugador2_C" (Transformation|GetWorldTransform (Variables|/Game/Blueprints/PJ_2.PJ_2_C|GetArrow (Variables|Default|GetPJ2))) "Undefined" 0 0)
        (bind _asgm_fuego_hielo (Utilities|Casting|CastToGM_FuegoHielo (Game|GetGameMode)))
        (Variables|/Game/Blueprints/GM_FuegoHielo.GM_FuegoHielo_C|SetTemperatura _asgm_fuego_hielo (+ (Variables|/Game/Blueprints/GM_FuegoHielo.GM_FuegoHielo_C|GetTemperatura _asgm_fuego_hielo) (Variables|Default|GetFuegesicto)))
        (Utilities|FlowControl|Delay 0.2)
        (Variables|Default|SetDisparoPJ2 false))))
  (:Released
    (Utilities|FlowControl|Delay 0.01)
    (goto _label Reset)))

(event Input|KeyboardEvents|S
  (params (Key :type Key%20Structure))
  (:Pressed
    (Variables|Default|Sets true)
    (Variables|Default|SetmovimientoPJ1 true))
  (:Released
    (Variables|Default|Sets false)
    (Variables|Default|SetmovimientoPJ1 false)))

(event Input|KeyboardEvents|A
  (params (Key :type Key%20Structure))
  (:Pressed
    (Variables|Default|Seta true)
    (Variables|Default|SetmovimientoPJ1 true))
  (:Released
    (Variables|Default|Seta false)
    (Variables|Default|SetmovimientoPJ1 false)))

(event Input|KeyboardEvents|D
  (params (Key :type Key%20Structure))
  (:Pressed
    (Variables|Default|Setd true)
    (Variables|Default|SetmovimientoPJ1 true))
  (:Released
    (Variables|Default|Setd false)
    (Variables|Default|SetmovimientoPJ1 false)))

(event Input|KeyboardEvents|Enter
  (params (Key :type Key%20Structure))
  (:Pressed
    (Variables|Default|SetDisparoPJ2 true)
    (Utilities|FlowControl|DoOnce false :!label _label
      (:Completed
        (Game|SpawnActorfromClass "/Game/Blueprints/ProyecticlJugador2.ProyecticlJugador2_C" (Transformation|GetWorldTransform (Variables|/Game/Blueprints/PJ_2.PJ_2_C|GetArrow (Variables|Default|GetPJ2))) "Undefined" 0 0)
        (bind _asgm_fuego_hielo (Utilities|Casting|CastToGM_FuegoHielo (Game|GetGameMode)))
        (Variables|/Game/Blueprints/GM_FuegoHielo.GM_FuegoHielo_C|SetTemperatura _asgm_fuego_hielo (+ (Variables|/Game/Blueprints/GM_FuegoHielo.GM_FuegoHielo_C|GetTemperatura _asgm_fuego_hielo) (Variables|Default|GetFuegesicto)))
        (Utilities|FlowControl|Delay 0.2)
        (Variables|Default|SetDisparoPJ2 false))))
  (:Released
    (Utilities|FlowControl|Delay 0.01)
    (goto _label Reset)))

(fn ConstructionScript)

(fn Jugador1alante
  (bind _refpj1 (Variables|Default|GetRefPJ1))
  (if (Variables|Default|Getw)
    (Utilities|IsValid _refpj1
      (:Is%20Valid
        (Transformation|AddActorWorldOffset _refpj1 (Math|Vector|MakeVector (+ (.x (Math|Vector|GetForwardVector (Variables|/Game/Blueprints/PJ_1n.PJ_1n_C|GetArrow _refpj1))) (Variables|Default|GetVelocidadJug)) 0.0 0.0) true)
        (Transformation|SetWorldRotation (Variables|/Script/Engine.Actor|GetRootComponent _refpj1) (Math|Rotator|MakeRotator 0.0 0.0 0.0) false false)))))

(fn Jugador1detras
  (bind _refpj1 (Variables|Default|GetRefPJ1))
  (if (Variables|Default|Gets)
    (Utilities|IsValid _refpj1
      (:Is%20Valid
        (Transformation|AddActorWorldOffset _refpj1 (Math|Vector|MakeVector (- (.x (Math|Vector|GetForwardVector (Variables|/Game/Blueprints/PJ_1n.PJ_1n_C|GetArrow _refpj1))) (Variables|Default|GetVelocidadJug)) 0.0 0.0) true)
        (Transformation|SetWorldRotation (Variables|/Script/Engine.Actor|GetRootComponent _refpj1) (Math|Rotator|MakeRotator 0.0 0.0 -1.8e+02) false false)))))

(fn Jugador1izquierda
  (bind _refpj1 (Variables|Default|GetRefPJ1))
  (if (Variables|Default|Geta)
    (Utilities|IsValid _refpj1
      (:Is%20Valid
        (Transformation|AddActorWorldOffset _refpj1 (Math|Vector|MakeVector 0.0 (- (.y (Math|Vector|GetForwardVector (Variables|/Game/Blueprints/PJ_1n.PJ_1n_C|GetArrow _refpj1))) (Variables|Default|GetVelocidadJug)) 0.0) true)
        (Transformation|SetWorldRotation (Variables|/Script/Engine.Actor|GetRootComponent _refpj1) (Math|Rotator|MakeRotator 0.0 0.0 -9e+01) false false)))))

(fn Jugador1derecha
  (bind _refpj1 (Variables|Default|GetRefPJ1))
  (if (Variables|Default|Getd)
    (Utilities|IsValid _refpj1
      (:Is%20Valid
        (Transformation|AddActorWorldOffset _refpj1 (Math|Vector|MakeVector 0.0 (+ (.y (Math|Vector|GetForwardVector (Variables|/Game/Blueprints/PJ_1n.PJ_1n_C|GetArrow _refpj1))) (Variables|Default|GetVelocidadJug)) 0.0) true)
        (Transformation|SetWorldRotation (Variables|/Script/Engine.Actor|GetRootComponent _refpj1) (Math|Rotator|MakeRotator 0.0 0.0 9e+01) false false)))))

(fn Jugador2derecha
  (bind _pj2 (Variables|Default|GetPJ2))
  (bind _pj2_2 (Variables|Default|GetPJ2))
  (if (Variables|Default|Getright)
    (Utilities|IsValid _pj2_2
      (:Is%20Valid
        (Transformation|AddActorWorldOffset _pj2 (Math|Vector|MakeVector 0.0 (+ (.y (Math|Vector|GetForwardVector (Variables|/Game/Blueprints/PJ_2.PJ_2_C|GetArrow _pj2_2))) (Variables|Default|GetVelocidadJug)) 0.0) true)
        (Transformation|SetWorldRotation (Variables|/Script/Engine.Actor|GetRootComponent _pj2) (Math|Rotator|MakeRotator 0.0 0.0 9e+01) false false)))))

(fn Jugador2izquierda
  (bind _pj2 (Variables|Default|GetPJ2))
  (bind _pj2_2 (Variables|Default|GetPJ2))
  (if (Variables|Default|Getizquierda)
    (Utilities|IsValid _pj2_2
      (:Is%20Valid
        (Transformation|AddActorWorldOffset _pj2 (Math|Vector|MakeVector 0.0 (- (.y (Math|Vector|GetForwardVector (Variables|/Game/Blueprints/PJ_2.PJ_2_C|GetArrow _pj2_2))) (Variables|Default|GetVelocidadJug)) 0.0) true)
        (Transformation|SetWorldRotation (Variables|/Script/Engine.Actor|GetRootComponent _pj2) (Math|Rotator|MakeRotator 0.0 0.0 -9e+01) false false)))))

(fn Jugador2abajo
  (bind _pj2 (Variables|Default|GetPJ2))
  (bind _pj2_2 (Variables|Default|GetPJ2))
  (if (Variables|Default|Getabajo)
    (Utilities|IsValid _pj2_2
      (:Is%20Valid
        (Transformation|AddActorWorldOffset _pj2 (Math|Vector|MakeVector (- (.x (Math|Vector|GetForwardVector (Variables|/Game/Blueprints/PJ_2.PJ_2_C|GetArrow _pj2_2))) (Variables|Default|GetVelocidadJug)) 0.0 0.0) true)
        (Transformation|SetWorldRotation (Variables|/Script/Engine.Actor|GetRootComponent _pj2) (Math|Rotator|MakeRotator 0.0 0.0 -1.8e+02) false false)))))

(fn Jugador2arriba
  (bind _pj2 (Variables|Default|GetPJ2))
  (bind _pj2_2 (Variables|Default|GetPJ2))
  (if (Variables|Default|Getarriba)
    (Utilities|IsValid _pj2_2
      (:Is%20Valid
        (Transformation|AddActorWorldOffset _pj2 (Math|Vector|MakeVector (+ (.x (Math|Vector|GetForwardVector (Variables|/Game/Blueprints/PJ_2.PJ_2_C|GetArrow _pj2_2))) (Variables|Default|GetVelocidadJug)) 0.0 0.0) true)
        (Transformation|SetWorldRotation (Variables|/Script/Engine.Actor|GetRootComponent _pj2) (Math|Rotator|MakeRotator 0.0 0.0 0.0) false false)))))

(fn Jugador1arribaderecha
  (bind _refpj1 (Variables|Default|GetRefPJ1))
  (bind _refpj1_2 (Variables|Default|GetRefPJ1))
  (bind _pj2 (Variables|Default|GetPJ2))
  (bind _pj2_2 (Variables|Default|GetPJ2))
  (bind _refpj1_3 (Variables|Default|GetRefPJ1))
  (bind _refpj1_4 (Variables|Default|GetRefPJ1))
  (bind _pj2_3 (Variables|Default|GetPJ2))
  (bind _pj2_4 (Variables|Default|GetPJ2))
  (Utilities|FlowControl|Sequence
    (:then_0
      (if (and (Variables|Default|Getd) (Variables|Default|Getw))
        (Utilities|IsValid _refpj1_2
          (:Is%20Valid
            (Transformation|SetWorldRotation (Variables|/Script/Engine.Actor|GetRootComponent _refpj1_2) (Math|Rotator|MakeRotator 0.0 0.0 45.0) false false)))))
    (:then_1
      (if (and (Variables|Default|Getd) (Variables|Default|Gets))
        (Utilities|IsValid _refpj1_3
          (:Is%20Valid
            (Transformation|SetWorldRotation (Variables|/Script/Engine.Actor|GetRootComponent _refpj1_3) (Math|Rotator|MakeRotator 0.0 0.0 135.0) false false)))))
    (:then_2
      (if (and (Variables|Default|Geta) (Variables|Default|Gets))
        (Utilities|IsValid _refpj1_4
          (:Is%20Valid
            (Transformation|SetWorldRotation (Variables|/Script/Engine.Actor|GetRootComponent _refpj1_4) (Math|Rotator|MakeRotator 0.0 0.0 -135.0) false false)))))
    (:then_3
      (if (and (Variables|Default|Geta) (Variables|Default|Getw))
        (Utilities|IsValid _refpj1
          (:Is%20Valid
            (Transformation|SetWorldRotation (Variables|/Script/Engine.Actor|GetRootComponent _refpj1) (Math|Rotator|MakeRotator 0.0 0.0 -45.0) false false)))))
    (:then_4
      (Utilities|FlowControl|Sequence
        (:then_0
          (if (and (Variables|Default|Getright) (Variables|Default|Getarriba))
            (Utilities|IsValid _pj2_3
              (:Is%20Valid
                (Transformation|SetWorldRotation (Variables|/Script/Engine.Actor|GetRootComponent _pj2_3) (Math|Rotator|MakeRotator 0.0 0.0 45.0) false false)))))
        (:then_1
          (if (and (Variables|Default|Getright) (Variables|Default|Getabajo))
            (Utilities|IsValid _pj2_2
              (:Is%20Valid
                (Transformation|SetWorldRotation (Variables|/Script/Engine.Actor|GetRootComponent _pj2_2) (Math|Rotator|MakeRotator 0.0 0.0 135.0) false false)))))
        (:then_2
          (if (and (Variables|Default|Getizquierda) (Variables|Default|Getabajo))
            (Utilities|IsValid _pj2
              (:Is%20Valid
                (Transformation|SetWorldRotation (Variables|/Script/Engine.Actor|GetRootComponent _pj2) (Math|Rotator|MakeRotator 0.0 0.0 -135.0) false false)))))
        (:then_3
          (if (and (Variables|Default|Getizquierda) (Variables|Default|Getarriba))
            (Utilities|IsValid _pj2_4
              (:Is%20Valid
                (Transformation|SetWorldRotation (Variables|/Script/Engine.Actor|GetRootComponent _pj2_4) (Math|Rotator|MakeRotator 0.0 0.0 -45.0) false false)))))))))
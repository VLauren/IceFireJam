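; Game mode for the two-player FuegoHielo game, handling spawning, lives, level progression and temperature visuals.
; BeginPlay creates HUD widgets, spawns both players at tagged points, registers them with Playersbutons and finds the level index in DataTable_Levels.
; The last enemy's death or LevelUP/LevelDOWN opens an adjacent table row's level; QuedanVidas? shows a paused death screen or respawns the flagged player after a delay.
; Tick maps Temperatura to stepped post-process stages.
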(event Custom|QuedanVidas?
  (if (<= (Variables|Default|GetVidas) 0)
    (Game|SetGamePaused true)
    (bind _returnvalue (UserInterface|CreateWidget "/Game/Widgets/Widg_End_Muerte.Widg_End_Muerte_C"))
    (UserInterface|Viewport|AddtoViewport _returnvalue 0)
    (elif (Variables|Default|GetPJ1)
      (Utilities|FlowControl|Delay 3.0)
      (bind _returnvalue_2 (Game|SpawnActorfromClass "/Game/Blueprints/PJ_1n.PJ_1n_C" (Math|Transform|MakeTransform (Variables|Default|GetLocationSpawn_1) "0, 0, 0" "1,1,1") "AdjustIfPossibleButAlwaysSpawn" 0 0))
      (Variables|Default|SetPJ1 false)
      (Variables|/Game/Blueprints/playersbutons.playersbutons_C|SetRefPJ1 (Variables|Default|GetRef_PLayerButtons) _returnvalue_2)
      (elif (Variables|Default|GetPJ2)
        (Utilities|FlowControl|Delay 3.0)
        (bind _returnvalue_3 (Game|SpawnActorfromClass "/Game/Blueprints/PJ_2.PJ_2_C" (Math|Transform|MakeTransform (Variables|Default|GetLocationSpawn_2) "0, 0, 0" "1,1,1") "AdjustIfPossibleButAlwaysSpawn" 0 0))
        (Variables|Default|SetPJ2 false)
        (Variables|/Game/Blueprints/playersbutons.playersbutons_C|SetPJ2 (Variables|Default|GetRef_PLayerButtons) _returnvalue_3)))))

(event Custom|Enemigo%20Muerto
  (bind _outactors (Actor|GetAllActorsOfClass "/Game/Blueprints/Enemies/ClasesNoColocables/Enemy.Enemy_C"))
  (if (== (- (Utilities|Array|Length _outactors) 1) 0)
    (Variables|Default|SetLevelSelected (+ (Variables|Default|GetLevelSelected) 1))
    (bind _outrownames (DataTable|GetDataTableRowNames "/Game/Data/DataTable_Levels.DataTable_Levels"))
    (Game|OpenLevel(byName) (Utilities|Array|Get(acopy) _outrownames (Variables|Default|GetLevelSelected)))))

(event Custom|LevelUP
  (Variables|Default|SetLevelSelected (+ (Variables|Default|GetLevelSelected) 1))
  (bind _outrownames (DataTable|GetDataTableRowNames "/Game/Data/DataTable_Levels.DataTable_Levels"))
  (Game|OpenLevel(byName) (Utilities|Array|Get(acopy) _outrownames (Variables|Default|GetLevelSelected))))

(event Custom|LevelDOWN
  (Variables|Default|SetLevelSelected (- (Variables|Default|GetLevelSelected) 1))
  (bind _outrownames (DataTable|GetDataTableRowNames "/Game/Data/DataTable_Levels.DataTable_Levels"))
  (Game|OpenLevel(byName) (Utilities|Array|Get(acopy) _outrownames (Variables|Default|GetLevelSelected))))

(event EventBeginPlay
  (bind _outactors (Actor|GetAllActorsOfClass "/Game/Blueprints/playersbutons.playersbutons_C"))
  (Variables|Default|SetRef_PLayerButtons (Utilities|Array|Get(acopy) _outactors))
  (bind _returnvalue (UserInterface|CreateWidget "/Game/Widgets/Widg_Temp.Widg_Temp_C"))
  (UserInterface|Viewport|AddtoViewport _returnvalue 0)
  (bind _returnvalue_2 (UserInterface|CreateWidget "/Game/Widgets/Widg_Vidas.Widg_Vidas_C"))
  (UserInterface|Viewport|AddtoViewport _returnvalue_2 0)
  (bind _outactors_2 (Actor|GetAllActorswithTag "SPAWN1"))
  (bind _output_get (Variables|Default|SetLocationSpawn_1 (Transformation|GetActorLocation (Utilities|Array|Get(acopy) _outactors_2))))
  (bind _returnvalue_3 (Game|SpawnActorfromClass "/Game/Blueprints/PJ_1n.PJ_1n_C" (Math|Transform|MakeTransform _output_get "0, 0, 0" "1,1,1") "AdjustIfPossibleButAlwaysSpawn" 0 0))
  (Variables|/Game/Blueprints/playersbutons.playersbutons_C|SetRefPJ1 (Variables|Default|GetRef_PLayerButtons) _returnvalue_3)
  (bind _outactors_3 (Actor|GetAllActorswithTag "SPAWN2"))
  (bind _output_get_2 (Variables|Default|SetLocationSpawn_2 (Transformation|GetActorLocation (Utilities|Array|Get(acopy) _outactors_3))))
  (bind _returnvalue_4 (Game|SpawnActorfromClass "/Game/Blueprints/PJ_2.PJ_2_C" (Math|Transform|MakeTransform _output_get_2 "0, 0, 0" "1,1,1") "AdjustIfPossibleButAlwaysSpawn" 0 0))
  (Variables|/Game/Blueprints/playersbutons.playersbutons_C|SetPJ2 (Variables|Default|GetRef_PLayerButtons) _returnvalue_4)
  (bind _outactors_4 (Actor|GetAllActorsOfClass "/Game/Blueprints/PostProcess.PostProcess_C"))
  (Variables|Default|SetPostProcess_ref (Utilities|Array|Get(acopy) _outactors_4))
  (bind _returnvalue_5 (Game|GetCurrentLevelName true))
  (bind _returnvalue_6 (Utilities|GetDataTableRow "/Game/Data/DataTable_Levels.DataTable_Levels" (Utilities|String|StringToName _returnvalue_5))
    (:then
      (Variables|Default|SetLevelSelected (.Index (Utilities|Struct|BreakStruct_Levels _returnvalue_6))))))

(event EventTick
  (params (DeltaSeconds :type Float%20%28single-precision%29))
  (bind _temperatura (Variables|Default|GetTemperatura))
  (bind _postprocess_ref (Variables|Default|GetPostProcess_ref))
  (bind _returnvalue (* _temperatura 1e+01))
  (if (== (Math|Float|Truncate _returnvalue) 0)
    (Variables|/Game/Blueprints/PostProcess.PostProcess_C|SetStage _postprocess_ref 0)
    (Default|StageUpdate _postprocess_ref :!label _label)
    (elif (== (Math|Float|Truncate _returnvalue) 1)
      (Variables|/Game/Blueprints/PostProcess.PostProcess_C|SetStage _postprocess_ref 1)
      (goto _label)
      (elif (== (Math|Float|Truncate _returnvalue) 2)
        (Variables|/Game/Blueprints/PostProcess.PostProcess_C|SetStage _postprocess_ref 2)
        (goto _label)
        (elif (== (Math|Float|Truncate _returnvalue) 3)
          (Variables|/Game/Blueprints/PostProcess.PostProcess_C|SetStage _postprocess_ref 3)
          (goto _label)
          (elif (== (Math|Float|Truncate _returnvalue) 4)
            (Variables|/Game/Blueprints/PostProcess.PostProcess_C|SetStage _postprocess_ref 4)
            (goto _label)
            (elif (== (Math|Float|Truncate _returnvalue) 5)
              (Variables|/Game/Blueprints/PostProcess.PostProcess_C|SetStage _postprocess_ref 5)
              (goto _label)
              (elif (== (Math|Float|Truncate _returnvalue) 6)
                (Variables|/Game/Blueprints/PostProcess.PostProcess_C|SetStage _postprocess_ref 6)
                (goto _label)
                (elif (== (Math|Float|Truncate _returnvalue) 7)
                  (Variables|/Game/Blueprints/PostProcess.PostProcess_C|SetStage _postprocess_ref 7)
                  (goto _label)
                  (elif (== (Math|Float|Truncate _returnvalue) 8)
                    (Variables|/Game/Blueprints/PostProcess.PostProcess_C|SetStage _postprocess_ref 8)
                    (goto _label)
                    (elif (== (Math|Float|Truncate _returnvalue) 9)
                      (Variables|/Game/Blueprints/PostProcess.PostProcess_C|SetStage _postprocess_ref 9)
                      (goto _label)
                      (elif (== (Math|Float|Truncate _returnvalue) 10)
                        (Variables|/Game/Blueprints/PostProcess.PostProcess_C|SetStage _postprocess_ref 10)
                        (goto _label)))))))))))))

(fn ConstructionScript)